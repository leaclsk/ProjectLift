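; BP_Lift is a lift actor that animates two door meshes, with travel between floors left unimplemented.
; Tick drives a FlipFlop that switches the Movement timeline between Play and Reverse every frame.
; The timeline sets both doors' relative Z and prints a debug "LiftOpen" message.
; The H key's CanOpen check and EventMove lead nowhere, and the random DestinationFloor pick is never executed.
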(event `Key|H`
  (params (Key :type "Key Structure"))
  (:`Pressed`
    (if (`self.CanOpen`)
      _)))

(event `EventMove`)

(event `self.ReceiveTick`
  (params (DeltaSeconds :type "Float (single-precision)"))
  (`/Engine/EditorBlueprintResources/StandardMacros.FlipFlop`
    (:`A`
      (bind (_direction _newtrack_0) (`Timeline|Movement` :!label _label)
        (:`Update`
          (`SceneComponent.K2_SetRelativeLocation` (`self.SM_Lift01Door2_StaticMeshComponent0`) (`KismetMathLibrary.MakeVector` 0.0 0.0 _newtrack_0) false false)
          (`SceneComponent.K2_SetRelativeLocation` (`self.SM_Lift01Door3_StaticMeshComponent0`) (`KismetMathLibrary.MakeVector` 0.0 0.0 _newtrack_0) false false)
          (`KismetSystemLibrary.PrintText` "LiftOpen"))))
    (:`B`
      (goto _label :!via `Reverse`))))

(fn `UserConstructionScript`)